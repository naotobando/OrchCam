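; Camera manager that switches the player's view between default pawn, auto orbit, free and saved fixed cameras through keyboard hotkeys.
; BeginPlay registers the pawn and a spawned orbit camera with BPCCameraStateController; the free camera spawns lazily at the current view on first use.
; BPCFixedCamModule saves fixed cameras captured from free-cam mode, recalled by number keys.
; Other keys vary the orbit and toggle a persistent camera shake by changing its scale.
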(event EventBeginPlay
  (bind _returnvalue (Game|Player|GetPlayerPawn 0))
  (Utilities|FlowControl|Sequence
    (:then_0
      (Utilities|IsValid _returnvalue
        (:Is%20Valid
          (Default|SetDefaultPawn (Variables|Default|GetBPC_CameraStateController) _returnvalue))
        (:Is%20Not%20Valid
          (Development|PrintString "DefaultPawn can not be found" false))))
    (:then_1
      ;[0.15 0.15 0.15 0.5] CameraShakeをInstanceする。開始時はScaleを0にしてOff
      ; On/Offは0キーで行う
      (bind _returnvalue_2 (CameraShakes|StartCameraShake (Variables|/Script/Engine.PlayerController|GetPlayerCameraManager (Game|GetPlayerController 0)) "/OrchCam/CharacterSet/CS_OrchCam.CS_OrchCam_C" 0.0 "CameraLocal" "0, 0, 0"))
      (Variables|Default|SetShakeInstance _returnvalue_2))
    (:then_2
      ;[0.15 0.15 0.15 0.5] OrbitCameraを生成し、StateControlleに登録
      (bind _returntransform (CallFunction|InitializeFreeCamTransform)) ; PlayerControllerの位置を返している\nDefaultPawnの有無などで位置を調整する関数
      (bind _returnvalue_3 (Game|SpawnActorfromClass "/OrchCam/CharacterSet/BP_OrbitCam.BP_OrbitCam_C" _returntransform "Undefined" "MultiplyWithRoot" 0 0))
      (bind _output_get (Variables|Default|SetOrbitCamRef _returnvalue_3))
      (Default|SetOrbitCamPawn (Variables|Default|GetBPC_CameraStateController) _output_get) ; StateControllerにOrbitCamを登録
    )))

(event Input|KeyboardEvents|RightBracket
  (params (Key :type Key%20Structure :default "None"))
  ;[0.15 0.15 0.15 0.5] ] : Autoカメラに切り替え
  (:Pressed
    (Default|ChangeCamState (Variables|Default|GetBPC_CameraStateController) "NewEnumerator1")))

(event Input|KeyboardEvents|Shift8
  (params (Key :type Key%20Structure :default "None"))
  (bind _shakeinstance (Variables|Default|GetShakeInstance))
  ;[0.15 0.15 0.15 0.5] CameraShakeのOn/Off
  (:Pressed
    (Utilities|FlowControl|FlipFlop
      (:A
        (Variables|/Script/Engine.CameraShakeBase|SetShakeScale _shakeinstance 1.0))
      (:B
        (Variables|/Script/Engine.CameraShakeBase|SetShakeScale _shakeinstance 0.0)))))

(event Input|KeyboardEvents|1
  (params (Key :type Key%20Structure :default "None"))
  ;[0.15 0.15 0.15 0.5] 0 ~ 9 : FixedCameraの呼び出し
  ; 実装的には10個以上のカメラも可能
  ; その場合は呼び出すイベントに手入れが必要
  (:Pressed
    (bind _keynumber (Utilities|SwitchFixedCam Key)
      (:execute2
        (CallFunction|SwitchtoFixedCambyIndex _keynumber)))))

(event Input|KeyboardEvents|2
  (params (Key :type Key%20Structure :default "None"))
  ;[0.15 0.15 0.15 0.5] 0 ~ 9 : FixedCameraの呼び出し
  ; 実装的には10個以上のカメラも可能
  ; その場合は呼び出すイベントに手入れが必要
  (:Pressed
    (bind _keynumber (Utilities|SwitchFixedCam Key)
      (:execute2
        (CallFunction|SwitchtoFixedCambyIndex _keynumber)))))

(event Input|KeyboardEvents|3
  (params (Key :type Key%20Structure :default "None"))
  ;[0.15 0.15 0.15 0.5] 0 ~ 9 : FixedCameraの呼び出し
  ; 実装的には10個以上のカメラも可能
  ; その場合は呼び出すイベントに手入れが必要
  (:Pressed
    (bind _keynumber (Utilities|SwitchFixedCam Key)
      (:execute2
        (CallFunction|SwitchtoFixedCambyIndex _keynumber)))))

(event Input|KeyboardEvents|4
  (params (Key :type Key%20Structure :default "None"))
  ;[0.15 0.15 0.15 0.5] 0 ~ 9 : FixedCameraの呼び出し
  ; 実装的には10個以上のカメラも可能
  ; その場合は呼び出すイベントに手入れが必要
  (:Pressed
    (bind _keynumber (Utilities|SwitchFixedCam Key)
      (:execute2
        (CallFunction|SwitchtoFixedCambyIndex _keynumber)))))

(event Input|KeyboardEvents|5
  (params (Key :type Key%20Structure :default "None"))
  ;[0.15 0.15 0.15 0.5] 0 ~ 9 : FixedCameraの呼び出し
  ; 実装的には10個以上のカメラも可能
  ; その場合は呼び出すイベントに手入れが必要
  (:Pressed
    (bind _keynumber (Utilities|SwitchFixedCam Key)
      (:execute2
        (CallFunction|SwitchtoFixedCambyIndex _keynumber)))))

(event Input|KeyboardEvents|6
  (params (Key :type Key%20Structure :default "None"))
  ;[0.15 0.15 0.15 0.5] 0 ~ 9 : FixedCameraの呼び出し
  ; 実装的には10個以上のカメラも可能
  ; その場合は呼び出すイベントに手入れが必要
  (:Pressed
    (bind _keynumber (Utilities|SwitchFixedCam Key)
      (:execute2
        (CallFunction|SwitchtoFixedCambyIndex _keynumber)))))

(event Input|KeyboardEvents|7
  (params (Key :type Key%20Structure :default "None"))
  ;[0.15 0.15 0.15 0.5] 0 ~ 9 : FixedCameraの呼び出し
  ; 実装的には10個以上のカメラも可能
  ; その場合は呼び出すイベントに手入れが必要
  (:Pressed
    (bind _keynumber (Utilities|SwitchFixedCam Key)
      (:execute2
        (CallFunction|SwitchtoFixedCambyIndex _keynumber)))))

(event Input|KeyboardEvents|8
  (params (Key :type Key%20Structure :default "None"))
  ;[0.15 0.15 0.15 0.5] 0 ~ 9 : FixedCameraの呼び出し
  ; 実装的には10個以上のカメラも可能
  ; その場合は呼び出すイベントに手入れが必要
  (:Pressed
    (bind _keynumber (Utilities|SwitchFixedCam Key)
      (:execute2
        (CallFunction|SwitchtoFixedCambyIndex _keynumber)))))

(event Input|KeyboardEvents|Shift0
  (params (Key :type Key%20Structure :default "None"))
  ;[0.15 0.15 0.15 0.5] Shift +0 : AutoCamのアングルを変更
  ; Shift +9 : AutoCamの距離を変更
  ; Shift + Space : AutoCameraのターゲット切り替え
  (:Pressed
    (Default|MovetoRadomOrbit (Variables|Default|GetOrbitCamRef))))

(event Input|KeyboardEvents|Shift9
  (params (Key :type Key%20Structure :default "None"))
  ;[0.15 0.15 0.15 0.5] Shift +0 : AutoCamのアングルを変更
  ; Shift +9 : AutoCamの距離を変更
  ; Shift + Space : AutoCameraのターゲット切り替え
  (:Pressed
    (Default|ChangeRandomDistance (Variables|Default|GetOrbitCamRef))))

(event Input|KeyboardEvents|ShiftSpaceBar
  (params (Key :type Key%20Structure :default "None"))
  ;[0.15 0.15 0.15 0.5] Shift +0 : AutoCamのアングルを変更
  ; Shift +9 : AutoCamの距離を変更
  ; Shift + Space : AutoCameraのターゲット切り替え
  (:Pressed
    (Default|SetNextTarget (Variables|Default|GetOrbitCamRef))))

(event Input|KeyboardEvents|L
  (params (Key :type Key%20Structure :default "None"))
  (bind _bpc_fixedcammodule (Variables|Default|GetBPC_FixedCamModule))
  ;[0.15 0.15 0.15 0.5] L : DebugModeの時のみDebugCamera位置にFixedCameraを追加
  ; Viewに変更はない
  (:Pressed
    (if (Utilities|Enum|Equal(Enum) (Variables|/OrchCam/CharacterSet/BPC_CameraStateController.BPC_CameraStateController_C|GetCurrentState (Variables|Default|GetBPC_CameraStateController)) "NewEnumerator2")
      (Default|AddFixedCamatCurrentView _bpc_fixedcammodule)
      (Default|SaveFixedCams _bpc_fixedcammodule))))

(event Input|KeyboardEvents|P
  (params (Key :type Key%20Structure :default "None"))
  ;[0.15 0.15 0.15 0.5] P : DefaultCameraに切り替え
  (:Pressed
    (Default|ChangeCamState (Variables|Default|GetBPC_CameraStateController) "NewEnumerator0")))

(event Input|KeyboardEvents|LeftBracket
  (params (Key :type Key%20Structure :default "None"))
  ;[0.15 0.15 0.15 0.5] [ : FreeCamを（初回）生成したり、FreeCamへ切り替えを行う
  (:Pressed
    (Utilities|IsValid (Variables|Default|GetFreeCamRef) ; Pを押したのが初回かどうか\nつまり初回なら各種初期化を実施
      (:Is%20Valid
        (Default|ChangeCamState (Variables|Default|GetBPC_CameraStateController) "NewEnumerator2"))
      (:Is%20Not%20Valid
        (bind _returntransform (CallFunction|InitializeFreeCamTransform)) ; defaultPawnがあるかどうかで\nカメラを向ける場所を変える
        (bind _returnvalue (Game|SpawnActorfromClass "/OrchCam/CharacterSet/BP_FreeCam.BP_FreeCam_C" _returntransform "Undefined" "MultiplyWithRoot" 0 0))
        (bind _output_get (Variables|Default|SetFreeCamRef _returnvalue))
        (Default|SetFreeCamPawn (Variables|Default|GetBPC_CameraStateController) _output_get) ; StateController側にDebugCameraを渡す
        (Default|ChangeCamState (Variables|Default|GetBPC_CameraStateController) "NewEnumerator2")))))

(event Input|KeyboardEvents|9
  (params (Key :type Key%20Structure :default "None"))
  ;[0.15 0.15 0.15 0.5] 0 ~ 9 : FixedCameraの呼び出し
  ; 実装的には10個以上のカメラも可能
  ; その場合は呼び出すイベントに手入れが必要
  (:Pressed
    (bind _keynumber (Utilities|SwitchFixedCam Key)
      (:execute2
        (CallFunction|SwitchtoFixedCambyIndex _keynumber)))))

(event Input|KeyboardEvents|0
  (params (Key :type Key%20Structure :default "None"))
  ;[0.15 0.15 0.15 0.5] 0 ~ 9 : FixedCameraの呼び出し
  ; 実装的には10個以上のカメラも可能
  ; その場合は呼び出すイベントに手入れが必要
  (:Pressed
    (bind _keynumber (Utilities|SwitchFixedCam Key)
      (:execute2
        (CallFunction|SwitchtoFixedCambyIndex _keynumber)))))

(fn ConstructionScript)

(fn InitializeFreeCamTransform
  (bind _returnvalue (Game|Player|GetPlayerPawn 0))
  (bind _returnvalue_2 (Actor|GetComponentbyClass _returnvalue "/Script/Engine.CameraComponent"))
  (Utilities|IsValid _returnvalue ; PossessしているPawnが存在するかどうか
    (:Is%20Valid
      (if (Utilities|IsValid _returnvalue_2)
        ;[0.15 0.15 0.15 0.5] Possessしているpawnがある＆Cameraコンポーネントがある場合
        ; Cameraコンポーネント位置&向きを返す（そこにDebugCamを作成する）
        (return (Transformation|GetWorldTransform _returnvalue_2))
        (else
          ;[0.15 0.15 0.15 0.5] PossessしているPawnがある＆Cameraコンポーネントがない場合
          ; Pawn位置＆Controller向きを返す（そこにDebugCamを作成する）
          (return (Math|Transform|MakeTransform (Transformation|GetActorLocation (Game|Player|GetPlayerPawn 0)) (Pawn|GetControlRotation (Game|GetPlayerController 0) :!class /Script/Engine.Controller))))))
    (:Is%20Not%20Valid
      ;[0.15 0.15 0.15 0.5] PossessしているPawnがない場合
      ; Controller位置&向きを返す（そこにDebugCamを作成する）
      (return (Transformation|GetActorTransform (Game|GetPlayerController 0))))))

(fn SwitchtoFixedCambyIndex
  (params (Index :type Integer))
  (if (Utilities|Array|IsValidIndex (Variables|/OrchCam/CharacterSet/BPC_FixedCamModule.BPC_FixedCamModule_C|GetFixedCamArray (Variables|Default|GetBPC_FixedCamModule)) Index)
    (Default|ChangeCamState (Variables|Default|GetBPC_CameraStateController) "NewEnumerator3" Index)))