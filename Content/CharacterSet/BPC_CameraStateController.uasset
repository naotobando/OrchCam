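; Camera state controller component that switches the player's view between default, orbit (Auto), free and fixed cameras, using pawns supplied through setter events.
; ChangeCamState stores the new state and blends the view target, taking indexed fixed cameras from the owner's BPC_FixedCamModule.
; Only Free possesses its own pawn.
; Leaving Free saves the control rotation and repossesses the default pawn, so re-entering restores the free camera's direction.
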(event Custom|SetDefaultPawn
  (params (DefaultPawn :type Pawn%20Object%20Reference))
  ;[0.15 0.15 0.15 0.5] BP_CameraManagerから呼び出す初期設定
  (Variables|Default|SetDefault%20Pawn DefaultPawn))

(event Custom|SetFreeCamPawn
  (params (FreeCam :type Pawn%20Object%20Reference))
  ;[0.15 0.15 0.15 0.5] BP_CameraManagerから呼び出す初期設定
  (Variables|Default|SetFree%20CamPawn FreeCam)
  (Variables|Default|SetFreeCamRotation (Pawn|GetControlRotation (Game|GetPlayerController 0) :!class /Script/Engine.Controller)))

(event Custom|SetOrbitCamPawn
  (params (OrbitCamPawn :type BP%20Orbit%20Cam%20Object%20Reference))
  ;[0.15 0.15 0.15 0.5] BP_CameraManagerから呼び出す初期設定
  (Variables|Default|SetOrbit%20Cam%20Pawn OrbitCamPawn))

(event Custom|ChangeCamState
  (params (NewState :type E_CameraState%20Enum :default "NewEnumerator0") (TargetIndex :type Integer))
  (Utilities|FlowControl|Sequence
    (:then_0
      (CallFunction|CheckStateIsFree) ; StateがFreeだった場合、カメラ向きを保存し、PossessをDefaultPawnにもどす\n他のstate場合はなにもしない
    )
    (:then_1
      (Variables|Default|SetCurrentState NewState))
    (:then_2
      (switch Utilities|FlowControl|Switch|SwitchonE_CameraState NewState
        (:NewEnumerator0
          (CallFunction|SetDefaultCamView))
        (:NewEnumerator1
          (CallFunction|SetOrbitCamView))
        (:NewEnumerator2
          (CallFunction|SetFreeCamView))
        (:NewEnumerator3
          (CallFunction|SetFixedCamView TargetIndex))))))

(event Custom|CheckStateIsFree
  (bind _returnvalue (Game|GetPlayerController 0))
  (bind _currentstate (Variables|Default|GetCurrentState))
  (bind _returnvalue_2 (Utilities|Enum|Equal(Enum) _currentstate "NewEnumerator2"))
  ;[0.15 0.15 0.15 0.5] 切り替え前のstateがFreeCamのとき、コントローラの向きを保存しDefaultPawnにPossessを渡す
  ;
  ; 背景：FreeCamのカメラ向きはActorではなくgame controllerの向き
  ; なので保存しないとFreeCamに戻した時に復元できなくなる
  (Development|PrintString (Utilities|String|ToString(Boolean) _returnvalue_2))
  (if _returnvalue_2
    (Variables|Default|SetFreeCamRotation (Pawn|GetControlRotation _returnvalue :!class /Script/Engine.Controller))
    (Pawn|Possess _returnvalue (Variables|Default|GetDefault%20Pawn))))

(event Custom|SetDefaultCamView
  ;[0.15 0.15 0.15 0.5] DefaultCamにカメラを切り替える
  ; PossessはDefaultPawn
  (Game|Player|SetViewTargetwithBlend (Game|GetPlayerController 0) (Variables|Default|GetDefault%20Pawn) 0.0 "VTBlend_Linear" 0.0 false))

(event Custom|SetOrbitCamView
  ;[0.15 0.15 0.15 0.5] OrbitCamにカメラを切り替える
  ; PossessはDefaultPawn
  (Game|Player|SetViewTargetwithBlend (Game|GetPlayerController 0) (Variables|Default|GetOrbit%20Cam%20Pawn) 0.0 "VTBlend_Linear" 0.0 false))

(event Custom|SetFreeCamView
  (bind _returnvalue (Game|GetPlayerController 0))
  (bind _free_campawn (Variables|Default|GetFree%20CamPawn))
  ;[0.15 0.15 0.15 0.5] FreeCamにカメラを切り替える
  ; PossessもFreeCamに変更
  (Pawn|Possess _returnvalue _free_campawn)
  (Pawn|SetControlRotation _returnvalue (Variables|Default|GetFreeCamRotation))
  (Game|Player|SetViewTargetwithBlend _returnvalue _free_campawn 0.0 "VTBlend_Linear" 0.0 false))

(event Custom|SetFixedCamView
  (params (TargetIndcex :type Integer))
  ;[0.15 0.15 0.15 0.5] FixedViewにカメラを切り替える
  ; PossessはDefaultPawn
  (Game|Player|SetViewTargetwithBlend (Game|GetPlayerController 0) (Utilities|Array|Get(acopy) (Variables|/OrchCam/CharacterSet/BPC_FixedCamModule.BPC_FixedCamModule_C|GetFixedCamArray (Actor|GetComponentbyClass (Components|GetOwner) "/OrchCam/CharacterSet/BPC_FixedCamModule.BPC_FixedCamModule_C")) TargetIndcex) 0.0 "VTBlend_Linear" 0.0 false))