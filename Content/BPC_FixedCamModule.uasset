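; BPC_FixedCamModule manages BP_FixedCam cameras and records their transforms for BP_CameraManager.
; On BeginPlay it indexes existing cameras by CameraIndex into FixedCamArray, then loads or creates the SG_CameraSave object.
; AddFixedCamAtCurrentView spawns a camera at the player's viewpoint, assigns its index, and appends the transform to the save object.
; SaveFixedCams writes that object to the slot; saved transforms are not respawned here.
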(event Custom|AddFixedCamAtCurrentView
  (bind _returnvalue (Game|GetPlayerController 0))
  (bind (_location _rotation) (Pawn|GetPlayerViewPoint _returnvalue))
  (bind _returnvalue_2 (Math|Transform|MakeTransform _location _rotation))
  (Utilities|FlowControl|Sequence
    (:then_0
      ;[0.15 0.15 0.15 0.5] 現在のプレイヤー位置にFixed Cameraをスポーンし、既存のカメラ配列に追加
      (bind _returnvalue_3 (Game|SpawnActorfromClass "/OrchCam/BP_FixedCam.BP_FixedCam_C" _returnvalue_2 "Undefined" "MultiplyWithRoot" 0 0))
      (bind _returnvalue_4 (Utilities|Array|Add (Variables|Default|GetFixedCamArray) _returnvalue_3))
      (Variables|/OrchCam/BP_FixedCam.BP_FixedCam_C|SetCameraIndex _returnvalue_3 _returnvalue_4))
    (:then_1
      ;[0.15 0.15 0.15 0.5] Fixed Cameraをspawnした位置をsave game objectに追加
      (Utilities|Array|Add (Variables|/OrchCam/SG_CameraSave.SG_CameraSave_C|GetSavedTransforms (Variables|Default|GetSaveGameObject)) _returnvalue_2))))

(event Custom|SaveFixedCams
  (bind _savegameobject (Variables|Default|GetSaveGameObject))
  ;[0.15 0.15 0.15 0.5] メモリ上のSaveGameObjectの内容を実際のデータとして書き出し
  (Utilities|IsValid _savegameobject
    (:Is%20Valid
      (SaveGame|SaveGametoSlot _savegameobject (Variables|Default|GetSaveSlotName)))))

(event EventBeginPlay
  (Utilities|FlowControl|Sequence
    (:then_0
      ;[0.15 0.15 0.15 0.5] Level内のBP_FixedCameraを配列に入れ、ゲーム再生時に再度SaveGameできるようにする
      ; これをしないと、EUWからカメラをレベルに追加した時に追加したカメラを再保存できない
      (bind _outactors (Actor|GetAllActorsOfClass "/OrchCam/BP_FixedCam.BP_FixedCam_C"))
      (for _array_element _outactors
        (Utilities|Array|SetArrayElem (Variables|Default|GetFixedCamArray) (Variables|/OrchCam/BP_FixedCam.BP_FixedCam_C|GetCameraIndex _array_element) _array_element true)))
    (:then_1
      ;[0.15 0.15 0.15 0.5] 起動時にセーブデータの有無を調べ、ロードまたはデータの作成を行う
      (bind _returnvalue (SaveGame|DoesSaveGameExist (Variables|Default|GetSaveSlotName))) ; 過去に保存したデータはあるかをチェック
      (if _returnvalue
        (bind _returnvalue_2 (SaveGame|LoadGamefromSlot (Variables|Default|GetSaveSlotName))) ; セーブデータがあるのでロードする
        (bind _assg_camera_save (Utilities|Casting|CastToSG_CameraSave _returnvalue_2))
        (Variables|Default|SetSaveGameObject _assg_camera_save)
        (else
          (bind _returnvalue_3 (SaveGame|CreateSaveGameObject "/OrchCam/SG_CameraSave.SG_CameraSave_C")) ; セーブデータがないので作成する
          (Variables|Default|SetSaveGameObject _returnvalue_3))))))