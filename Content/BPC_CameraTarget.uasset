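; BPC_CameraTarget is a scene component that makes its owning actor a target for BP_OrbitCam.
; It registers the owner on BeginPlay under its display name and unregisters it on EndPlay.
; Both steps find the camera with GetActorOfClass, retry next frame if none exists, and print debug messages.
; A separate SetInitialTarget event makes the owner the camera's initial target, without retrying.
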(event Custom|RegisterToOrbitCam
  (bind _returnvalue (Components|GetOwner))
  (bind _returnvalue_2 (Utilities|GetDisplayName _returnvalue))
  ;[0.15 0.15 0.15 0.5] このSceneComponentをつけられているアクターをOrbitCamに登録する
  (bind _returnvalue_3 (Actor|GetActorOfClass "/OrchCam/BP_OrbitCam.BP_OrbitCam_C"))
  (Utilities|IsValid _returnvalue_3
    (:Is%20Valid
      (Default|RegisterTarget _returnvalue_3 (Utilities|String|StringToName _returnvalue_2) _returnvalue)
      (Development|PrintString (Utilities|String|Append _returnvalue_2 " : RegisterToOrbitCam") false))
    (:Is%20Not%20Valid
      (Utilities|FlowControl|DelayUntilNextFrame)
      (CallFunction|RegistertoOrbitCam)
      (Development|PrintString (Utilities|String|Append _returnvalue_2 " : Can not find OrbitCam") false))))

(event Custom|UnregisterFromOrbitCam
  ;[0.15 0.15 0.15 0.5] アクターが削除される時に、OrbitCamからActorの登録を解除する
  (bind _returnvalue (Actor|GetActorOfClass "/OrchCam/BP_OrbitCam.BP_OrbitCam_C"))
  (Utilities|IsValid _returnvalue
    (:Is%20Valid
      (Default|UnregisterTarget _returnvalue (Utilities|String|StringToName (Utilities|GetDisplayName (Components|GetOwner))))
      (Development|PrintString "UnregisterFromOrbitCam" false))
    (:Is%20Not%20Valid
      (Utilities|FlowControl|DelayUntilNextFrame)
      (CallFunction|UnregisterfromOrbitCam)
      (Development|PrintString "Can not find OrbitCam" false))))

(event Custom|SetInitialTarget
  ;[0.15 0.15 0.15 0.5] 初期設定したいBPの場合はこれを呼ぶ必要がある
  (bind _returnvalue (Actor|GetActorOfClass "/OrchCam/BP_OrbitCam.BP_OrbitCam_C"))
  (Utilities|IsValid _returnvalue
    (:Is%20Valid
      (Default|SetInitialTarget _returnvalue (Components|GetOwner)))))

(event EventBeginPlay
  (CallFunction|RegistertoOrbitCam))

(event EventEndPlay
  (params (EndPlayReason :type EEndPlayReason%20Enum :default "Destroyed"))
  (CallFunction|UnregisterfromOrbitCam))