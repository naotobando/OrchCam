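; BP_OrbitCam is a single camera that follows one subject at a time and moves around it.
; Tick interpolates its root toward the target plus an offset from BPC_CameraTarget or actor bounds, picking a random target if none is valid.
; Subjects register in TargetMap, allowing switching by random pick, next, ID or index.
; Callable events use timelines to lerp the SpringArm to random rotations and distances, timed by MoveDuration.
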(event Custom|SetTrackingTarget
  (params (NewTarget :type Actor%20Object%20Reference))
  ;[0.15 0.15 0.15 0.5] 撮影対象の変更
  ; BP_OrbitCamは一つのカメラで被写体の周りを動き回る
  ; 被写体の特定の位置を映すため、被写体変更時に今の被写体と映したい場所の位置差分を計算している
  (bind _output_get (Variables|Default|SetTargetActor NewTarget))
  (Variables|Default|SetTargetDistanceFromOrigin (CallFunction|CalculateTargetOffset _output_get)))

(event Custom|MoveToRadomOrbit
  (bind _pitchrange (Variables|Default|GetPitchRange))
  ;[0.15 0.15 0.15 0.5] TargetActorの周辺をランダムに動き回るイベント
  (Utilities|FlowControl|Sequence
    (:then_0
      (Variables|Default|SetStartRotation (Variables|/Script/Engine.SceneComponent|GetRelativeRotation (Variables|Default|GetSpringArm))) ; SpringArmの初期値を保存
      (Variables|Default|SetTargetRotation (Math|Rotator|MakeRotator (Math|Random|RandomFloatinRange -45.0 45.0) (Math|Random|RandomFloatinRange (.x _pitchrange) (.y _pitchrange)) (Math|Random|RandomFloatinRange 0.0 3.6e+02))) ; ランダムに作成したSpringArmのターゲット値を保存
    )
    (:then_1
      (Components|Timeline|SetPlayRate (Variables|Default|GetTL_Rotation) (/ 1.0 (Variables|Default|GetMoveDuration))) ; MoveDurationが大きくなると\n動きがゆっくりになる
      (bind _newtrack_0 (Timeline|TL_Rotation PlayFromStart)
        (:Update
          (Transformation|SetRelativeRotation (Variables|Default|GetSpringArm) (Math|Rotator|Lerp(Rotator) (Variables|Default|GetStartRotation) (Variables|Default|GetTargetRotation) _newtrack_0 true) false true))))))

(event Custom|ChangeRandomDistance
  ;[0.15 0.15 0.15 0.5] TargetActorのに対し、カメラ位置を近づけたり遠ざけたりす
  (Utilities|FlowControl|Sequence
    (:then_0
      (Variables|Default|SetStartLength (Variables|/Script/Engine.SpringArmComponent|GetTargetArmLength (Variables|Default|GetSpringArm)))
      (Variables|Default|SetTargetLength (Math|Random|RandomFloatinRange (Variables|Default|GetMinDistance) (Variables|Default|GetMaxDistance))))
    (:then_1
      (Components|Timeline|SetPlayRate (Variables|Default|GetTL_Distance) (/ 1.0 (Variables|Default|GetMoveDuration)))
      (bind _newtrack_0 (Timeline|TL_Distance PlayFromStart)
        (:Update
          (Variables|/Script/Engine.SpringArmComponent|SetTargetArmLength (Variables|Default|GetSpringArm) (Math|Float|Lerp (Variables|Default|GetStartLength) (Variables|Default|GetTargetLength) _newtrack_0)))))))

(event Custom|RegisterTarget
  (params (TargetID :type Name) (Actor :type Actor%20Object%20Reference))
  ;[0.15 0.15 0.15 0.5] 被写体に設定したBPC_TargetCameraから呼ばれるイベント。
  ; すべての被写体を格納する。
  (Utilities|Map|Add (Variables|Default|GetTargetMap) TargetID Actor))

(event Custom|SetRandomTarget
  ;[0.15 0.15 0.15 0.5] 別の被写体にカメラを向ける際に利用する関数群
  (bind _randomtarget (CallFunction|GetRandomTarget)) ; Mapの中からランダムでターゲットのActorを返す
  (CallFunction|SetTrackingTarget _randomtarget))

(event Custom|SetNextTarget
  ;[0.15 0.15 0.15 0.5] 別の被写体にカメラを向ける際に利用する関数群
  (bind _necxttarget (CallFunction|GetNextTarget)) ; Mapの次の要素を返す\n最後に達した場合は最初に戻る
  (CallFunction|SetTrackingTarget _necxttarget))

(event Custom|SetTargetByID
  (params (RequestedID :type Name))
  ;[0.15 0.15 0.15 0.5] 別の被写体にカメラを向ける際に利用する関数群
  (bind _requestedtarget (CallFunction|GetTargetbyID RequestedID)) ; Map内のkeyのActorを返す
  (CallFunction|SetTrackingTarget _requestedtarget))

(event Custom|SetTargetByIndex
  (params (RequestedIndex :type Integer))
  ;[0.15 0.15 0.15 0.5] 別の被写体にカメラを向ける際に利用する関数群
  (bind _requestedtarget (CallFunction|GetTargetbyIndex RequestedIndex)) ; 指定のIndexのActorを返す
  (CallFunction|SetTrackingTarget _requestedtarget))

(event Custom|UnregisterTarget
  (params (TargetID :type Name%20%28by%20ref%29))
  ;[0.15 0.15 0.15 0.5] 被写体がdestoryされる時にmapから削除する
  (Utilities|Map|Remove (Variables|Default|GetTargetMap) TargetID))

(event Custom|SetInitialTarget
  (params (TargetActor :type Actor%20Object%20Reference))
  ;[0.15 0.15 0.15 0.5] 初期ターゲットにしたいActorから呼ぶ
  (Variables|Default|SetTargetActor TargetActor))

(event EventTick
  (params (DeltaSeconds :type Float%20%28single-precision%29))
  (bind _targetactor (Variables|Default|GetTargetActor))
  ;[0.15 0.15 0.15 0.5] 被写体が移動した時にゆっくりと追いかけるようにする
  (Utilities|IsValid _targetactor ; 基本的にはActor側からこのBPのSetInitialTargetが\n呼ばれるのが期待値それがない場合は、適当に選択
    (:Is%20Valid
      (Transformation|SetWorldLocation (Variables|Default|GetDefaultSceneRoot) (Math|Interpolation|VInterpTo (Transformation|GetActorLocation) (+ (Transformation|GetActorLocation _targetactor) (Variables|Default|GetTargetDistanceFromOrigin)) (Utilities|Time|GetWorldDeltaSeconds) (Variables|Default|GetTrackingSpeed)) false false) ; このBP（カメラ）自身の位置を更新
    )
    (:Is%20Not%20Valid
      (CallFunction|SetRandomTarget))))

(fn ConstructionScript)

(fn CalculateTargetOffset
  (params (TargetActor :type Actor%20Object%20Reference))
  (bind _returnvalue (Actor|GetComponentsByClass TargetActor "/OrchCam/BPC_CameraTarget.BPC_CameraTarget_C"))
  (bind _returnvalue_2 (Transformation|GetActorLocation TargetActor))
  (bind (_origin _boxextent) (Collision|GetActorBounds TargetActor true false))
  (bind (_x _y _z) (Math|Vector|BreakVector _returnvalue_2))
  ;[0.15 0.15 0.15 0.5] 渡されたActorがBPC_CameraTargetを持つときは、BPC_CameraTargetの位置とActor本体との位置差分を返す
  (if (> (Utilities|Array|Length _returnvalue) 0)
    (return (- (Transformation|GetWorldLocation (Utilities|Array|Get(acopy) _returnvalue)) _returnvalue_2))
    (else
      ;[0.15 0.15 0.15 0.5] 渡されたActorがBPC_CameraTargetを持たないとき、ActorのBoundsの中心より少し上とのActor本体との位置差分を返す
      (return (- (Math|Vector|MakeVector _x _y (+ (.Z (Math|Vector|BreakVector _origin)) (* (.z _boxextent) 0.5))) (Math|Vector|MakeVector _x _y _z))))))

(fn GetRandomTarget
  (bind _keys (Utilities|Map|Keys (Variables|Default|GetTargetMap)))
  (return (.Value (Utilities|Map|GetKeyValueByIndex (Variables|Default|GetTargetMap) (Math|Random|RandomIntegerinRange 0 (Utilities|Array|LastIndex _keys))))))

(fn GetNextTarget
  (Utilities|FlowControl|Sequence
    (:then_0
      ;[0.15 0.15 0.15 0.5] currentTargetIndexをmapの要素数内でインクリメント
      (bind _keys (Utilities|Map|Keys (Variables|Default|GetTargetMap)))
      (bind _result (Math|Integer|IncrementInt (Variables|Default|GetCurrentTargetIndex))
        (:%20%20
          (Variables|Default|SetCurrentTargetIndex (Math|Integer|%(Integer) _result (Utilities|Array|Length _keys))))))
    (:then_1
      ;[0.15 0.15 0.15 0.5] インクリメントしたIndexを使って要素を返す
      (return (.Value (Utilities|Map|GetKeyValueByIndex (Variables|Default|GetTargetMap) (Variables|Default|GetCurrentTargetIndex)))))))

(fn GetTargetbyID
  (params (RequestedID :type Name%20%28by%20ref%29))
  (bind _targetmap (Variables|Default|GetTargetMap))
  (bind (_value _returnvalue) (Utilities|Map|Find _targetmap RequestedID))
  (if _returnvalue ; RequestedIDがない場合には逃がす
    (return _value)
    (else
      (Development|PrintString "Called GetNextTargetByID, but ID is not found." false))))

(fn GetTargetbyIndex
  (params (RequestedIndex :type Integer))
  (if (> (Utilities|Map|Length (Variables|Default|GetTargetMap)) RequestedIndex) ; 引数がLengthより小さければtrue
    (return (.Value (Utilities|Map|GetKeyValueByIndex (Variables|Default|GetTargetMap) RequestedIndex)))
    (else
      (Development|PrintString "Called GetNextTargetByIndex, but Index is not found." false))))